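; MineGames sets up four-player local multiplayer for MineRush.
; On BeginPlay it reuses or creates local players, assigns each MineCont a PlayerID, destroys its pawn, calls Init with itself, then forces effects, texture and material quality through console commands.
; MovePlayersToSpawn, not called here, teleports each controller's pawn to the SpawnPoint whose PlayerSpawnID matches its PlayerID, found by FindSpawnPoint.
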(event EventBeginPlay
  (bind _returnvalue (Game|GetPlayerController 0))
  (Utilities|FlowControl|Sequence
    (:then_0
      (bind _returnvalue_2 (Class|GameMode|GetNumPlayers))
      (if (== _returnvalue_2 4)
        (for _index (range 0 3)
          (bind _asmine_cont (Utilities|Casting|CastToMineCont (Game|GetPlayerController _index)))
          (Variables|/Game/MineRush/Blueprints/Character/MineCont.MineCont_C|SetPlayer%20ID _asmine_cont _index)
          (Utilities|IsValid (Pawn|GetControlledPawn _asmine_cont)
            (:Is%20Valid
              (Actor|DestroyActor (Pawn|GetControlledPawn _asmine_cont)))))
        (else
          (for _index_2 (range 1 4)
            (bind _returnvalue_3 (Class|GameplayStatics|CreatePlayer -1))
            (bind _asmine_cont_2 (Utilities|Casting|CastToMineCont _returnvalue_3))
            (Variables|/Game/MineRush/Blueprints/Character/MineCont.MineCont_C|SetPlayer%20ID _asmine_cont_2 _index_2)
            (Utilities|IsValid (Pawn|GetControlledPawn _asmine_cont_2)
              (:Is%20Valid
                (Actor|DestroyActor (Pawn|GetControlledPawn _asmine_cont_2)))))))
      (bind _outactors (Actor|GetAllActorsOfClass "/Game/MineRush/Blueprints/Character/MineCont.MineCont_C"))
      (for _array_element _outactors
        (Default|Init _array_element self)))
    (:then_1
      (Development|ExecuteConsoleCommand "sg.EffectsQuality 3" _returnvalue)
      (Development|ExecuteConsoleCommand "sg.TextureQuality 3" _returnvalue)
      (Development|ExecuteConsoleCommand "r.MaterialQualityLevel 3" _returnvalue))))

(fn ConstructionScript)

(fn FindSpawnPoint
  (params (Player%20ID :type Integer))
  (bind _outactors (Actor|GetAllActorsOfClass "/Game/MineRush/Blueprints/Core/SpawnPoint.SpawnPoint_C"))
  (bind _array_element (Utilities|Array|ForEachLoopwithBreak _outactors :!label _label)
    (:LoopBody
      (if (== (Variables|/Game/MineRush/Blueprints/Core/SpawnPoint.SpawnPoint_C|GetPlayer%20Spawn%20ID _array_element) Player%20ID)
        (LocalVariables|SettempLocation (Transformation|GetActorLocation _array_element))
        (goto _label Break)))
    (:Completed
      (return (LocalVariables|GettempLocation)))))

(fn MovePlayerstoSpawn
  (bind _outactors (Actor|GetAllActorsOfClass "/Game/MineRush/Blueprints/Character/MineCont.MineCont_C"))
  (for _array_element _outactors
    (bind _spawn_loc (CallFunction|FindSpawnPoint (Variables|/Game/MineRush/Blueprints/Character/MineCont.MineCont_C|GetPlayer%20ID _array_element)))
    (Transformation|Teleport (Pawn|GetControlledPawn _array_element) _spawn_loc "0, 0, 0")))