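; Slot machine pickup in MineRush that turns into a random item when the side-scroller character overlaps its box.
; A chain of branches, each with a fresh random roll, favors earlier items among the eight pickups and restarts if all miss.
; The chosen pickup spawns at the transform saved on BeginPlay, then the machine destroys itself.
; Tick compares player distance to a glow threshold, but both greater and less results enable custom depth.
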(event OnComponentBeginOverlap(Box)
  (params (OtherActor :type Actor%20Object%20Reference) (OtherComp :type Primitive%20Component%20Object%20Reference) (OtherBodyIndex :type Integer) (bFromSweep :type Boolean) (SweepResult :type Hit%20Result%20Structure%20%28by%20ref%29))
  (bind _returnvalue (Math|Random|RandomIntegerinRange 0 7))
  (Utilities|Casting|CastToSideScrollerCharacter OtherActor)
  (if (== _returnvalue 0) :!label _label
    (Game|SpawnActorfromClass "/Game/MineRush/Blueprints/Pick_Ups/dynamitePickp.DynamitePickp_C" (Variables|Default|GetWorldTransform) "Undefined" 0 0)
    (elif (== _returnvalue 1)
      (Game|SpawnActorfromClass "/Game/MineRush/Blueprints/Pick_Ups/Feather.Feather_C" (Variables|Default|GetWorldTransform) "Undefined" 0 0)
      (elif (== _returnvalue 2)
        (Game|SpawnActorfromClass "/Game/MineRush/Blueprints/Pick_Ups/Green_Pocket_watch.Green_Pocket_watch_C" (Variables|Default|GetWorldTransform) "Undefined" 0 0)
        (elif (== _returnvalue 3)
          (Game|SpawnActorfromClass "/Game/MineRush/Blueprints/Pick_Ups/Red_Pocket_watch.Red_Pocket_watch_C" (Variables|Default|GetWorldTransform) "Undefined" 0 0)
          (elif (== _returnvalue 4)
            (Game|SpawnActorfromClass "/Game/MineRush/Blueprints/Pick_Ups/LunchBOx.LunchBox_C" (Variables|Default|GetWorldTransform) "Undefined" 0 0)
            (elif (== _returnvalue 5)
              (Game|SpawnActorfromClass "/Game/MineRush/Blueprints/Pick_Ups/BundleDynamitePickup.BundleDynamitePickup_C" (Variables|Default|GetWorldTransform) "Undefined" 0 0)
              (elif (== _returnvalue 6)
                (Game|SpawnActorfromClass "/Game/MineRush/Blueprints/Pick_Ups/Gaint_Spring_Pickup.Gaint_Spring_Pickup_C" (Variables|Default|GetWorldTransform) "Undefined" 0 0)
                (elif (== _returnvalue 7)
                  (Game|SpawnActorfromClass "/Game/MineRush/Blueprints/Pick_Ups/Alcohol.Alcohol_C" (Variables|Default|GetWorldTransform) "Undefined" 0 0)
                  (else
                    (goto _label))))))))))
  (Actor|DestroyActor))

(event EventBeginPlay
  (Variables|Default|SetWorldTransform (Transformation|GetWorldTransform (Variables|Default|GetDefaultSceneRoot))))

(event EventTick
  (params (DeltaSeconds :type Float%20%28single-precision%29))
  (Math|Float|CompareFloat (Transformation|GetDistanceTo (Game|GetPlayerCharacter 0)) (Variables|Default|GetDistForGlow)
    (:>
      _)
    (:<
      _))
  (Rendering|SetRenderCustomDepth (Variables|Default|GetSkeletalMesh) true))

(fn ConstructionScript)