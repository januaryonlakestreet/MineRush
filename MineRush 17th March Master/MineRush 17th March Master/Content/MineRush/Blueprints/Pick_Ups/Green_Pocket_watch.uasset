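; Green pocket watch pickup that speeds up the side-scroller character on contact.
; A Rotate timeline, started on BeginPlay, spins the actor by lerping between start and end rotations.
; Box overlap with a SideScrollerCharacter calls SPeedUP on it and destroys the pickup.
; Tick compares player distance to a glow threshold, but both greater and less branches enable custom depth on the Cone, never disabling it.
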(event OnComponentBeginOverlap(Box)
  (params (OtherActor :type Actor%20Object%20Reference) (OtherComp :type Primitive%20Component%20Object%20Reference) (OtherBodyIndex :type Integer) (bFromSweep :type Boolean) (SweepResult :type Hit%20Result%20Structure%20%28by%20ref%29))
  (bind _asside_scroller_character (Utilities|Casting|CastToSideScrollerCharacter OtherActor))
  (Default|SPeedUP _asside_scroller_character)
  (Actor|DestroyActor))

(event EventBeginPlay
  (bind _rot (Timeline|Rotate Play)
    (:Update
      (Transformation|SetActorRelativeRotation (Math|Rotator|Lerp(Rotator) (Variables|Default|GetStart) (Variables|Default|GetEnd) _rot)))))

(event EventTick
  (params (DeltaSeconds :type Float%20%28single-precision%29))
  (Math|Float|CompareFloat (Transformation|GetDistanceTo (Game|GetPlayerCharacter 0)) (Variables|Default|GetDistForGlow)
    (:>
      _)
    (:<
      _))
  (Rendering|SetRenderCustomDepth (Variables|Default|GetCone) true))

(fn ConstructionScript)