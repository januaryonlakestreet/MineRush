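; Thrown dynamite projectile Blueprint that explodes and damages nearby actors tagged "Destroy".
; A sphere overlap starts a one-second fuse, then a multi sphere trace around the actor applies damage to each tagged hit.
; Only a tagged hit triggers Thrown, which removes the mesh, shows the explosion flipbook with sound, then destroys the actor.
; Tick holds the flipbook at a fixed world rotation.
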(event OnComponentBeginOverlap(Sphere)
  (params (OtherActor :type Actor%20Object%20Reference) (OtherComp :type Primitive%20Component%20Object%20Reference) (OtherBodyIndex :type Integer) (bFromSweep :type Boolean) (SweepResult :type Hit%20Result%20Structure%20%28by%20ref%29))
  (bind _returnvalue (Transformation|GetActorLocation))
  (bind (_x _y _z) (Math|Vector|BreakVector _returnvalue))
  ;[1 1 1] Function works need to make projectile
  (Utilities|FlowControl|Delay 1.0)
  (bind _outhits (Class|KismetSystemLibrary|SphereTraceMultiNEW _returnvalue (Math|Vector|MakeVector _x (+ _y 0.1) _z) 1e+02 "TraceTypeQuery1" false 0 "None" true))
  (bind _array_element (Utilities|Array|ForEachLoopwithBreak _outhits)
    (:LoopBody
      (if (Actor|ActorHasTag (.HitActor (Collision|BreakHitResult _array_element)) "Destroy")
        (Game|Damage|ApplyDamage (.HitActor (Collision|BreakHitResult _array_element)) 1e+02 0 0)
        (CallFunction|Thrown)))))

(event Custom|Thrown
  (Components|DestroyComponent (Variables|Default|GetStaticMesh))
  (Sprite|SetFlipbook (Variables|Default|GetFlipbookExplosive) "/Game/MineRush/ParticleSystems/ParticleFlipbooks/ExploFB.ExploFB")
  (Audio|PlaySoundatLocation "/Game/MineRush/Audio/S15_DynamitePickup_3_.S15_DynamitePickup_3_" (Transformation|GetActorLocation))
  (Utilities|FlowControl|Delay 0.5)
  (Actor|DestroyActor))

(event EventTick
  (params (DeltaSeconds :type Float%20%28single-precision%29))
  ;[1 1 1] Function works need to make projectile
  (Transformation|SetWorldRotation (Variables|Default|GetFlipbookExplosive) "0,-90.000000, 0" false false))

(fn ConstructionScript)