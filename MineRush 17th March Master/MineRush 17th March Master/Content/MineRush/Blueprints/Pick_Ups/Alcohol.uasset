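; Alcohol pickup that inverts the player's left/right controls for five seconds.
; A timeline started on BeginPlay rotates the pickup.
; Box overlap by a SideScrollerCharacter destroys box and mesh, sets Inverted and swaps the Y of MineCont's movement vectors, then reverts them after a delay and destroys the actor.
; Tick compares player distance to DistForGlow, but both greater and less branches enable custom depth, so the glow never switches off.
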(event OnComponentBeginOverlap(Box)
  (params (OtherActor :type Actor%20Object%20Reference) (OtherComp :type Primitive%20Component%20Object%20Reference) (OtherBodyIndex :type Integer) (bFromSweep :type Boolean) (SweepResult :type Hit%20Result%20Structure%20%28by%20ref%29))
  (Utilities|Casting|CastToSideScrollerCharacter OtherActor)
  (bind _asmine_cont (Utilities|Casting|CastToMineCont (Game|GetPlayerController 0)))
  (Components|DestroyComponent (Variables|Default|GetBox))
  (Variables|/Game/MineRush/Blueprints/Character/MineCont.MineCont_C|SetInverted? _asmine_cont true)
  (Variables|/Game/MineRush/Blueprints/Character/MineCont.MineCont_C|SetMovement%20Vector%20Right _asmine_cont (Math|Vector|MakeVector (.X (Math|Vector|BreakVector (Variables|/Game/MineRush/Blueprints/Character/MineCont.MineCont_C|GetMovement%20Vector%20Right _asmine_cont))) (Variables|Default|Getinvert) (.Z (Math|Vector|BreakVector (Variables|/Game/MineRush/Blueprints/Character/MineCont.MineCont_C|GetMovement%20Vector%20Right _asmine_cont)))))
  (Variables|/Game/MineRush/Blueprints/Character/MineCont.MineCont_C|SetMovement%20Vector%20Left _asmine_cont (Math|Vector|MakeVector (.X (Math|Vector|BreakVector (Variables|/Game/MineRush/Blueprints/Character/MineCont.MineCont_C|GetMovement%20Vector%20Left _asmine_cont))) (Variables|Default|GetInvert%20Left) (.Z (Math|Vector|BreakVector (Variables|/Game/MineRush/Blueprints/Character/MineCont.MineCont_C|GetMovement%20Vector%20Left _asmine_cont)))))
  (Utilities|FlowControl|Delay 5.0)
  (Variables|/Game/MineRush/Blueprints/Character/MineCont.MineCont_C|SetInverted? _asmine_cont false)
  (Variables|/Game/MineRush/Blueprints/Character/MineCont.MineCont_C|SetMovement%20Vector%20Left _asmine_cont (Math|Vector|MakeVector (.X (Math|Vector|BreakVector (Variables|/Game/MineRush/Blueprints/Character/MineCont.MineCont_C|GetMovement%20Vector%20Left _asmine_cont))) (Variables|Default|GetrevertedLeft) (.Z (Math|Vector|BreakVector (Variables|/Game/MineRush/Blueprints/Character/MineCont.MineCont_C|GetMovement%20Vector%20Left _asmine_cont)))))
  (Variables|/Game/MineRush/Blueprints/Character/MineCont.MineCont_C|SetMovement%20Vector%20Right _asmine_cont (Math|Vector|MakeVector (.X (Math|Vector|BreakVector (Variables|/Game/MineRush/Blueprints/Character/MineCont.MineCont_C|GetMovement%20Vector%20Right _asmine_cont))) (Variables|Default|Getreverted) (.Z (Math|Vector|BreakVector (Variables|/Game/MineRush/Blueprints/Character/MineCont.MineCont_C|GetMovement%20Vector%20Right _asmine_cont)))))
  (Actor|DestroyActor))

(event EventBeginPlay
  ;[1 1 1] Pick Up Rotation
  (bind _rot (Timeline|Timeline_0 Play)
    (:Update
      (Transformation|SetActorRelativeRotation (Math|Rotator|Lerp(Rotator) (Variables|Default|GetStart) (Variables|Default|GetEnd) _rot)))))

(event EventTick
  (params (DeltaSeconds :type Float%20%28single-precision%29))
  (Math|Float|CompareFloat (Transformation|GetDistanceTo (Game|GetPlayerCharacter 0)) (Variables|Default|GetDistForGlow)
    (:>
      _)
    (:<
      _))
  (Rendering|SetRenderCustomDepth (Variables|Default|GetStaticMesh) true))

(fn ConstructionScript)