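; RandomPickup is a MineRush placeholder actor that spawns one of nine pickups at its root transform on BeginPlay, from dynamite to a slot machine.
; A chain of branches each makes a fresh random roll against its own index, looping back to the start if none match.
; Because the rolls are independent, pickups earlier in the chain are more likely to spawn.
; The placeholder stays in the level after spawning.
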(event EventBeginPlay
  (bind _returnvalue (Math|Random|RandomIntegerinRange 0 8))
  (Variables|Default|SetWorldTransform (Transformation|GetWorldTransform (Variables|Default|GetDefaultSceneRoot)))
  (if (== _returnvalue 0) :!label _label
    (Game|SpawnActorfromClass "/Game/MineRush/Blueprints/Pick_Ups/dynamitePickp.DynamitePickp_C" (Variables|Default|GetWorldTransform) "Undefined" 0 0)
    (elif (== _returnvalue 1)
      (Game|SpawnActorfromClass "/Game/MineRush/Blueprints/Pick_Ups/Feather.Feather_C" (Variables|Default|GetWorldTransform) "Undefined" 0 0)
      (elif (== _returnvalue 2)
        (Game|SpawnActorfromClass "/Game/MineRush/Blueprints/Pick_Ups/Green_Pocket_watch.Green_Pocket_watch_C" (Variables|Default|GetWorldTransform) "Undefined" 0 0)
        (elif (== _returnvalue 3)
          (Game|SpawnActorfromClass "/Game/MineRush/Blueprints/Pick_Ups/Red_Pocket_watch.Red_Pocket_watch_C" (Variables|Default|GetWorldTransform) "Undefined" 0 0)
          (elif (== _returnvalue 4)
            (Game|SpawnActorfromClass "/Game/MineRush/Blueprints/Pick_Ups/LunchBOx.LunchBox_C" (Variables|Default|GetWorldTransform) "Undefined" 0 0)
            (elif (== _returnvalue 5)
              (Game|SpawnActorfromClass "/Game/MineRush/Blueprints/Pick_Ups/BundleDynamitePickup.BundleDynamitePickup_C" (Variables|Default|GetWorldTransform) "Undefined" 0 0)
              (elif (== _returnvalue 6)
                (Game|SpawnActorfromClass "/Game/MineRush/Blueprints/Pick_Ups/Gaint_Spring_Pickup.Gaint_Spring_Pickup_C" (Variables|Default|GetWorldTransform) "Undefined" 0 0)
                (elif (== _returnvalue 7)
                  (Game|SpawnActorfromClass "/Game/MineRush/Blueprints/Pick_Ups/Alcohol.Alcohol_C" (Variables|Default|GetWorldTransform) "Undefined" 0 0)
                  (elif (== _returnvalue 8)
                    (Game|SpawnActorfromClass "/Game/MineRush/Blueprints/Pick_Ups/SlotMachine.SlotMachine_C" (Variables|Default|GetWorldTransform) "Undefined" 0 0)
                    (else
                      (goto _label))))))))))))

(fn ConstructionScript)