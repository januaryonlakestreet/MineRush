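; Patrolling AI for the MineRush side-scroller that walks back and forth at half input along the Y axis.
; Its Left and Right triggers react to "Block"-tagged actors by yawing the mesh and, after a short delay, setting the walk direction.
; The same triggers call StopMovement on any SideScrollerCharacter they overlap.
; Incoming damage lowers AIHealth and destroys the actor at zero or below.
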(event OnComponentBeginOverlap(Right)
  (params (OtherActor :type Actor%20Object%20Reference) (OtherComp :type Primitive%20Component%20Object%20Reference) (OtherBodyIndex :type Integer) (bFromSweep :type Boolean) (SweepResult :type Hit%20Result%20Structure%20%28by%20ref%29))
  (bind _mesh (Variables|Character|GetMesh))
  (bind _returnvalue (Transformation|GetWorldRotation _mesh))
  (bind (_roll _pitch _yaw) (Math|Rotator|BreakRotator _returnvalue))
  (Utilities|FlowControl|Sequence
    (:then_0
      (if (Actor|ActorHasTag OtherActor "Block")
        (Transformation|SetWorldRotation _mesh (Math|Rotator|MakeRotator _roll _pitch (- _yaw 9e+01)) false false)
        (Utilities|FlowControl|Delay 0.2)
        (Variables|Default|SetWalk%20direction "0,1.000000, 0")))
    (:then_1
      (bind _asside_scroller_character (Utilities|Casting|CastToSideScrollerCharacter OtherActor))
      (Default|StopMovement _asside_scroller_character))))

(event OnComponentBeginOverlap(Left)
  (params (OtherActor :type Actor%20Object%20Reference) (OtherComp :type Primitive%20Component%20Object%20Reference) (OtherBodyIndex :type Integer) (bFromSweep :type Boolean) (SweepResult :type Hit%20Result%20Structure%20%28by%20ref%29))
  (bind _mesh (Variables|Character|GetMesh))
  (bind _returnvalue (Transformation|GetWorldRotation _mesh))
  (bind (_roll _pitch _yaw) (Math|Rotator|BreakRotator _returnvalue))
  (Utilities|FlowControl|Sequence
    (:then_0
      (if (Actor|ActorHasTag OtherActor "Block")
        (Transformation|SetWorldRotation _mesh (Math|Rotator|MakeRotator _roll _pitch (- _yaw 9e+01)) false false)
        (Utilities|FlowControl|Delay 0.2)
        (Variables|Default|SetWalk%20direction "0,-1.000000, 0")))
    (:then_1
      (bind _asside_scroller_character (Utilities|Casting|CastToSideScrollerCharacter OtherActor))
      (Default|StopMovement _asside_scroller_character))))

(event EventBeginPlay
  (Variables|Default|SetTags (Variables|Default|GetTag)))

(event EventTick
  (params (DeltaSeconds :type Float%20%28single-precision%29))
  (Pawn|Input|AddMovementInput self (Variables|Default|GetWalk%20direction) 0.5 false))

(event Game|Damage|EventAnyDamage
  (params (Damage :type Float%20%28single-precision%29) (DamageType :type Damage%20Type%20Object%20Reference) (InstigatedBy :type Controller%20Object%20Reference) (DamageCauser :type Actor%20Object%20Reference))
  (Variables|Default|SetDamaged Damage)
  (Variables|Default|SetAIHealth (- (Variables|Default|GetAIHealth) (Variables|Default|GetDamaged)))
  (if (<= (Variables|Default|GetAIHealth) 0.0)
    (Actor|DestroyActor)))

(fn ConstructionScript)

(fn INIT
  (params (Controller :type Mine%20Cont%20Object%20Reference))
  (Variables|Default|SetOwningCont Controller))

(fn Health)