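; Two-way teleporter actor for the side-scroller character in MineRush, with a Sphere end and a Cylinder end.
; Overlapping either end line-traces beside the other, destroys the MineBlock it hits and teleports the character into that spot, after a short delay on the Sphere side.
; No teleport happens without a MineBlock hit.
; A Teleported flag, cleared one second after each jump, blocks immediate re-triggering.
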(event OnComponentBeginOverlap(Sphere)
  (params (OtherActor :type Actor%20Object%20Reference) (OtherComp :type Primitive%20Component%20Object%20Reference) (OtherBodyIndex :type Integer) (bFromSweep :type Boolean) (SweepResult :type Hit%20Result%20Structure%20%28by%20ref%29))
  (bind _cylinder (Variables|Default|GetCylinder))
  (bind _returnvalue (Transformation|GetWorldLocation _cylinder))
  (bind _returnvalue_2 (- _returnvalue "0,100.000000,25.000000"))
  (if (not (Variables|Default|GetTeleported))
    (bind _asside_scroller_character (Utilities|Casting|CastToSideScrollerCharacter OtherActor))
    (bind _outhit (Collision|LineTraceByChannel _returnvalue _returnvalue_2 "TraceTypeQuery1" false 0 "None"))
    (bind _asmine_block (Utilities|Casting|CastToMineBlock (.HitActor (Collision|BreakHitResult _outhit)))
      (:then
        (Actor|DestroyActor _asmine_block)
        (Utilities|FlowControl|Delay 0.2)
        (Transformation|Teleport _asside_scroller_character _returnvalue_2 "0, 0, 0")
        (Variables|Default|SetTeleported true)
        (Utilities|FlowControl|Delay 1.0)
        (Variables|Default|SetTeleported false))
      (:CastFailed
        (Development|PrintString "Hello")))))

(event OnComponentBeginOverlap(Cylinder)
  (params (OtherActor :type Actor%20Object%20Reference) (OtherComp :type Primitive%20Component%20Object%20Reference) (OtherBodyIndex :type Integer) (bFromSweep :type Boolean) (SweepResult :type Hit%20Result%20Structure%20%28by%20ref%29))
  (bind _sphere (Variables|Default|GetSphere))
  (bind _returnvalue (Transformation|GetWorldLocation _sphere))
  (bind _returnvalue_2 (- _returnvalue "0,-100.000000,-30.000000"))
  (if (not (Variables|Default|GetTeleported))
    (bind _asside_scroller_character (Utilities|Casting|CastToSideScrollerCharacter OtherActor))
    (bind _outhit (Collision|LineTraceByChannel _returnvalue _returnvalue_2 "TraceTypeQuery1" false 0 "None"))
    (bind _asmine_block (Utilities|Casting|CastToMineBlock (.HitActor (Collision|BreakHitResult _outhit))))
    (Actor|DestroyActor _asmine_block)
    (Transformation|Teleport _asside_scroller_character _returnvalue_2 "0, 0, 0")
    (Variables|Default|SetTeleported true)
    (Utilities|FlowControl|Delay 1.0)
    (Variables|Default|SetTeleported false)))

(fn ConstructionScript)