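; Stalagmite hazard for MineRush that calls the side-scroller character's Stalagmite handler when it overlaps the spike box.
; On BeginPlay a short downward line trace from the arrow identifies the mine, gold or explosive block beneath and caches it by type.
; Tick polls that block's health and destroys the stalagmite when it reaches zero.
; Any damage caused by the player character also destroys it.
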(event OnComponentBeginOverlap(SpikeBox)
  (params (OtherActor :type Actor%20Object%20Reference) (OtherComp :type Primitive%20Component%20Object%20Reference) (OtherBodyIndex :type Integer) (bFromSweep :type Boolean) (SweepResult :type Hit%20Result%20Structure%20%28by%20ref%29))
  (bind _asside_scroller_character (Utilities|Casting|CastToSideScrollerCharacter OtherActor))
  (Default|Stalagmite _asside_scroller_character))

(event EventBeginPlay
  (bind _arrow (Variables|Default|GetArrow))
  (bind _returnvalue (Transformation|GetWorldLocation _arrow))
  (bind (_x _y _z) (Math|Vector|BreakVector _returnvalue))
  (Variables|Default|SetTags (Variables|Default|GetTag))
  (bind (_outhit _returnvalue_2) (Collision|LineTraceByChannel _returnvalue (Math|Vector|MakeVector _x _y (- _z 1e+02)) "TraceTypeQuery1" false 0 "None"))
  (if _returnvalue_2
    (bind _asmine_block (Utilities|Casting|CastToMineBlock (.HitActor (Collision|BreakHitResult _outhit)))
      (:then
        (Variables|Default|SetBlock%20Below%20Type 0)
        (Variables|Default|SetNearest%20Mine%20Block _asmine_block))
      (:CastFailed
        (bind _asgold_block (Utilities|Casting|CastToGoldBLock (.HitActor (Collision|BreakHitResult _outhit)))
          (:then
            (Variables|Default|SetBlock%20Below%20Type 1)
            (Variables|Default|SetNearest%20Gold%20Block _asgold_block))
          (:CastFailed
            (bind _asexplosive (Utilities|Casting|CastToExplosive (.HitActor (Collision|BreakHitResult _outhit))))
            (Variables|Default|SetBlock%20Below%20Type 2)
            (Variables|Default|SetNearest%20Explosive%20Block _asexplosive)))))
    (else
      (Utilities|IsValid 0))))

(event Game|Damage|EventAnyDamage
  (params (Damage :type Float%20%28single-precision%29) (DamageType :type Damage%20Type%20Object%20Reference) (InstigatedBy :type Controller%20Object%20Reference) (DamageCauser :type Actor%20Object%20Reference))
  (Utilities|Casting|CastToSideScrollerCharacter DamageCauser)
  (Actor|DestroyActor))

(event EventTick
  (params (DeltaSeconds :type Float%20%28single-precision%29))
  (switch int (Variables|Default|GetBlock%20Below%20Type)
    (:0
      (if (== (Variables|/Game/MineRush/Blueprints/MineBlocks/MineBLock.MineBlock_C|GetBlockHealth (Variables|Default|GetNearest%20Mine%20Block)) 0.0)
        (Actor|DestroyActor)))
    (:1
      (if (== (Variables|/Game/MineRush/Blueprints/MineBlocks/GoldBLock.GoldBLock_C|GetBlockHealth (Variables|Default|GetNearest%20Gold%20Block)) 0.0)
        (Actor|DestroyActor)))
    (:2
      (if (== (Variables|/Game/MineRush/Blueprints/MineBlocks/Explosive.Explosive_C|GetBlockHealth (Variables|Default|GetNearest%20Explosive%20Block)) 0.0)
        (Actor|DestroyActor)))))

(fn ConstructionScript)