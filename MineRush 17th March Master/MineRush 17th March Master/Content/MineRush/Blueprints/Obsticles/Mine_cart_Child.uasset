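; Mine cart obstacle child Blueprint for MineRush that sets its own start and end locations before running the parent's logic.
; After a one-second delay, BeginPlay stores the capsule's world location as StartLoc and derives EndLOC at a fixed offset along negative Y.
; It waits another second before calling the parent BeginPlay, so both points are set first.
; The construction script only calls the parent's.
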(event EventBeginPlay
  (Utilities|FlowControl|Delay 1.0)
  (Variables|Default|SetStart%20Loc (Transformation|GetWorldLocation (Variables|Default|GetCapsuleComponent)))
  (Variables|Default|SetEnd%20LOC (- (Variables|Default|GetStart%20Loc) "0,1860.000000, 0"))
  (Utilities|FlowControl|Delay 1.0)
  (|CallParentFunction))

(fn ConstructionScript
  (|CallParentFunction))