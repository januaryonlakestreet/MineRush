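; Falling stalactite hazard for MineRush that drops when the player enters its Box trigger or when the block above it breaks.
; BeginPlay traces up to cache a mine, gold or explosive block, and Tick polls its health to start Timeline_0, while the trigger plays a separate Drop timeline.
; SpikeBox hits on MineBlocks or the player stop only Drop, show a rock flipbook and destroy it; player damage destroys it immediately.
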(event OnComponentBeginOverlap(SpikeBox)
  (params (OtherActor :type Actor%20Object%20Reference) (OtherComp :type Primitive%20Component%20Object%20Reference) (OtherBodyIndex :type Integer) (bFromSweep :type Boolean) (SweepResult :type Hit%20Result%20Structure%20%28by%20ref%29))
  (Utilities|FlowControl|Sequence
    (:then_0
      (Utilities|Casting|CastToMineBlock OtherActor)
      (Audio|Components|Audio|Stop (Variables|Default|GetDrop))
      (Rendering|SetVisibility (Variables|Default|GetStaticMesh1) false false)
      (Collision|SetCollisionEnabled (Variables|Default|GetSpikeBox) "NoCollision")
      (Sprite|SetFlipbook (Variables|Default|GetPaperFlipbook) "/Game/MineRush/ParticleSystems/ParticleFlipbooks/RockFB.RockFB")
      (Utilities|FlowControl|Delay 0.6)
      (Actor|DestroyActor))
    (:then_1
      (bind _asside_scroller_character (Utilities|Casting|CastToSideScrollerCharacter OtherActor))
      (Default|StopMovement _asside_scroller_character)
      (Audio|Components|Audio|Stop (Variables|Default|GetDrop))
      (Rendering|SetVisibility (Variables|Default|GetStaticMesh1) false false)
      (Collision|SetCollisionEnabled (Variables|Default|GetSpikeBox) "NoCollision")
      (Sprite|SetFlipbook (Variables|Default|GetPaperFlipbook) "/Game/MineRush/ParticleSystems/ParticleFlipbooks/RockFB.RockFB")
      (Utilities|FlowControl|Delay 0.6)
      (Actor|DestroyActor))))

(event OnComponentBeginOverlap(Box)
  (params (OtherActor :type Actor%20Object%20Reference) (OtherComp :type Primitive%20Component%20Object%20Reference) (OtherBodyIndex :type Integer) (bFromSweep :type Boolean) (SweepResult :type Hit%20Result%20Structure%20%28by%20ref%29))
  (bind _staticmesh6 (Variables|Default|GetStaticMesh6))
  (bind _returnvalue (Transformation|GetWorldLocation _staticmesh6))
  (Utilities|Casting|CastToSideScrollerCharacter OtherActor)
  (Class|KismetSystemLibrary|CapsuleTraceSingleforObjects _returnvalue (+ _returnvalue "0, 0,500.000000") 1e+01 1e+01 (Utilities|Array|MakeArray "ObjectTypeQuery3") false 0 "None" true)
  (Collision|SetCollisionEnabled (Variables|Default|GetBox) "NoCollision")
  (bind _newtrack_1 (Timeline|Drop Play)
    (:Update
      (Transformation|SetActorRelativeLocation (+ _newtrack_1 (Variables|Default|GetStart_Location)))
      (Utilities|FlowControl|Delay 6.0)
      (Actor|DestroyActor))))

(event EventTick
  (params (DeltaSeconds :type Float%20%28single-precision%29))
  (switch int (Variables|Default|GetBlock%20Above%20Type)
    (:0
      (if (== (Variables|/Game/MineRush/Blueprints/MineBlocks/MineBLock.MineBlock_C|GetBlockHealth (Variables|Default|GetNearest%20Mine%20Block)) 0.0)
        (bind _newtrack_1 (Timeline|Timeline_0 Play)
          (:Update
            (Transformation|SetActorRelativeLocation (+ _newtrack_1 (Variables|Default|GetStart_Location)))
            (Utilities|FlowControl|Delay 6.0)
            (Actor|DestroyActor)))))
    (:1
      (if (== (Variables|/Game/MineRush/Blueprints/MineBlocks/GoldBLock.GoldBLock_C|GetBlockHealth (Variables|Default|GetNearest%20Gold%20Block)) 0.0)
        (Timeline|Timeline_0 Play)))
    (:2
      (if (== (Variables|/Game/MineRush/Blueprints/MineBlocks/Explosive.Explosive_C|GetBlockHealth (Variables|Default|GetNearest%20Explosive%20Block)) 0.0)
        (Timeline|Timeline_0 Play)))))

(event Game|Damage|EventAnyDamage
  (params (Damage :type Float%20%28single-precision%29) (DamageType :type Damage%20Type%20Object%20Reference) (InstigatedBy :type Controller%20Object%20Reference) (DamageCauser :type Actor%20Object%20Reference))
  (Utilities|Casting|CastToSideScrollerCharacter DamageCauser)
  (Actor|DestroyActor))

(event EventBeginPlay
  (bind _arrow (Variables|Default|GetArrow))
  (bind _returnvalue (Transformation|GetWorldLocation _arrow))
  (bind (_x _y _z) (Math|Vector|BreakVector _returnvalue))
  (Utilities|FlowControl|Sequence
    (:then_0
      (bind (_outhit _returnvalue_2) (Collision|LineTraceByChannel _returnvalue (Math|Vector|MakeVector _x _y (+ _z 1e+02)) "TraceTypeQuery1" false 0 "ForDuration"))
      (if _returnvalue_2
        (bind _asmine_block (Utilities|Casting|CastToMineBlock (.HitActor (Collision|BreakHitResult _outhit)))
          (:then
            (Variables|Default|SetBlock%20Above%20Type 0)
            (Variables|Default|SetNearest%20Mine%20Block _asmine_block))
          (:CastFailed
            (bind _asgold_block (Utilities|Casting|CastToGoldBLock (.HitActor (Collision|BreakHitResult _outhit)))
              (:then
                (Variables|Default|SetBlock%20Above%20Type 1)
                (Variables|Default|SetNearest%20Gold%20Block _asgold_block))
              (:CastFailed
                (bind _asexplosive (Utilities|Casting|CastToExplosive (.HitActor (Collision|BreakHitResult _outhit))))
                (Variables|Default|SetBlock%20Above%20Type 2)
                (Variables|Default|SetNearest%20Explosive%20Block _asexplosive)))))
        (else
          (Utilities|IsValid 0))))
    (:then_1
      (Variables|Default|SetStart_Location (Transformation|GetWorldLocation (Variables|Default|GetDefaultSceneRoot))))))

(fn ConstructionScript)