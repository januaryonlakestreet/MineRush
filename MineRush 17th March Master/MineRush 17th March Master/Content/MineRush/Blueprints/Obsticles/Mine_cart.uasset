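; Mine cart obstacle that travels along a fixed path and knocks the side-scroller character aside.
; After a short delay on BeginPlay it plays a cart sound, then a Timeline lerps it along negative Y from its capsule's start location and destroys it when finished.
; Left and Right overlap components launch the character upward and in opposite Y directions.
; INIT stores an owning controller reference.
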(event OnComponentBeginOverlap(Right)
  (params (OtherActor :type Actor%20Object%20Reference) (OtherComp :type Primitive%20Component%20Object%20Reference) (OtherBodyIndex :type Integer) (bFromSweep :type Boolean) (SweepResult :type Hit%20Result%20Structure%20%28by%20ref%29))
  (bind _asside_scroller_character (Utilities|Casting|CastToSideScrollerCharacter OtherActor))
  (Character|LaunchCharacter _asside_scroller_character "0.000000,-800.000000,300.000000" false false))

(event OnComponentBeginOverlap(Left)
  (params (OtherActor :type Actor%20Object%20Reference) (OtherComp :type Primitive%20Component%20Object%20Reference) (OtherBodyIndex :type Integer) (bFromSweep :type Boolean) (SweepResult :type Hit%20Result%20Structure%20%28by%20ref%29))
  (bind _asside_scroller_character (Utilities|Casting|CastToSideScrollerCharacter OtherActor))
  (Character|LaunchCharacter _asside_scroller_character "0.000000,800.000000,300.000000" false false))

(event EventBeginPlay
  (Utilities|FlowControl|Delay 1.0)
  (Variables|Default|SetStart%20Loc (Transformation|GetWorldLocation (Variables|Collision|GetCapsuleComponent)))
  (Variables|Default|SetEnd%20LOC (- (Variables|Default|GetStart%20Loc) "0,2100.000000, 0"))
  (Audio|PlaySoundatLocation "/Game/MineRush/Audio/S12_CartObstacle.S12_CartObstacle" (Transformation|GetActorLocation))
  (bind _cameracurve (Timeline|Timeline_0 Play)
    (:Update
      (Transformation|SetActorRelativeLocation (Math|Vector|Lerp(Vector) (Variables|Default|GetStart%20Loc) (Variables|Default|GetEnd%20LOC) _cameracurve)))
    (:Finished
      (Actor|DestroyActor))))

(fn ConstructionScript)

(fn INIT
  (params (Controller :type Mine%20Cont%20Object%20Reference))
  (Variables|Default|SetOwningCont Controller))