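; MineBlock is a breakable block actor for MineRush that cracks as it takes damage and is destroyed at zero health.
; On BeginPlay, Small blocks roll one of three stone types, which sets health and dynamic material textures; gold is defined but never rolled.
; Row and column material parameters derive from the offset to the Is00 origin block.
; Damage updates the crack level, then death plays a rock flipbook before destroying the actor.
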(event Custom|Destroy
  ;[1 1 1] Andy's Flipbook Test Stuff
  (Components|DestroyComponent (Variables|Default|GetCube))
  (Sprite|SetFlipbook (Variables|Default|GetFlipbook%20Rock) "/Game/MineRush/ParticleSystems/ParticleFlipbooks/RockFB.RockFB"))

(event EventBeginPlay
  (bind _self self)
  (bind _defaultsceneroot (Variables|Default|GetDefaultSceneRoot _self))
  (bind _returnvalue (Transformation|GetWorldTransform _defaultsceneroot))
  (bind (_x _y _z) (Math|Vector|BreakVector (.location _returnvalue)))
  (Variables|Default|SetTags (Variables|Default|GetTag))
  (bind _outactors (Actor|GetAllActorsOfClass "MineBlock_C"))
  (bind _array_element (Utilities|Array|ForEachLoopwithBreak _outactors :!label _label)
    (:LoopBody
      (if (Variables|MineBlock_C|GetIs%2000 _array_element)
        (Variables|Default|Setblock00 _array_element)
        (goto _label Break)))
    (:Completed
      (if (Variables|Default|GetSmall)
        (bind _output_get (Variables|Default|SetRandomMAterial (Math|Random|RandomIntegerinRange 0 2)))
        (Variables|Default|SetBlockHealth (Math|Conversions|ToFloat(Integer) (+ _output_get 1)))
        (bind _returnvalue_2 (Rendering|Material|CreateDynamicMaterialInstance (Variables|Default|GetCube) 0 "/Game/MineRush/Materials/BackgroundMaster.BackgroundMaster" :!class /Script/Engine.PrimitiveComponent))
        (Rendering|Material|SetScalarParameterValue _returnvalue_2 "Column" (/ (- _y (.Y (Math|Vector|BreakVector (.location (Transformation|GetWorldTransform (Variables|MineBlock_C|GetDefaultSceneRoot (Variables|Default|Getblock00))))))) -1e+02) :!class /Script/Engine.MaterialInstanceDynamic)
        (Rendering|Material|SetTextureParameterValue _returnvalue_2 "TypeMaterial" (Utilities|Select :Index _output_get :Option%200 "/Game/MineRush/Materials/Textures/StoneSmall.StoneSmall" :Option%201 "/Game/MineRush/Materials/Textures/StoneMedium.StoneMedium" :Option%202 "/Game/MineRush/Materials/Textures/StoneBig.StoneBig" :Option%203 "/Game/MineRush/Materials/Textures/Gold.Gold"))
        (Rendering|Material|SetTextureParameterValue _returnvalue_2 "TypeMaterialNormal" (Utilities|Select :Index _output_get :Option%200 "/Game/MineRush/Materials/Textures/StoneSmall_Normal.StoneSmall_Normal" :Option%201 "/Game/MineRush/Materials/Textures/StoneMedium_Normal.StoneMedium_Normal" :Option%202 "/Game/MineRush/Materials/Textures/StoneBig_Normal.StoneBig_Normal" :Option%203 "/Game/MineRush/Materials/Textures/Gold_Normal.Gold_Normal"))
        (Rendering|Material|SetScalarParameterValue _returnvalue_2 "Row" (/ (- _z (.Z (Math|Vector|BreakVector (.location (Transformation|GetWorldTransform (Variables|MineBlock_C|GetDefaultSceneRoot (Variables|Default|Getblock00))))))) -1e+02) :!class /Script/Engine.MaterialInstanceDynamic)
        (Rendering|Material|SetScalarParameterValue _returnvalue_2 "IsItGold" (Math|Conversions|ToFloat(Integer) (select (== _output_get 3) 1 0)) :!class /Script/Engine.MaterialInstanceDynamic)
        (Rendering|Material|SetScalarParameterValue _returnvalue_2 "Specular" (/ (Math|Conversions|ToFloat(Integer) (select (== _output_get 3) 10 3)) 1e+01) :!class /Script/Engine.MaterialInstanceDynamic)
        (Rendering|Material|SetScalarParameterValue _returnvalue_2 "Roughness" (/ (Math|Conversions|ToFloat(Integer) (select (== _output_get 3) 2 3)) 1e+01) :!class /Script/Engine.MaterialInstanceDynamic)))))

(event Game|Damage|EventAnyDamage
  (params (Damage :type Float%20%28single-precision%29) (DamageType :type Damage%20Type%20Object%20Reference) (InstigatedBy :type Controller%20Object%20Reference) (DamageCauser :type Actor%20Object%20Reference))
  ;[1 1 1] Damage/Health
  (Variables|Default|SetDamaged Damage)
  ;[1 1 1] Block Crack
  (Rendering|Material|SetScalarParameterValue (stale EventBeginPlay _returnvalue_2) "Crack_Level" (Math|Conversions|ToFloat(Integer) (+ (select (<= (/ (* (Variables|Default|GetBlockHealth) 1e+02) (Math|Conversions|ToFloat(Integer) (+ (stale EventBeginPlay _output_get) 1))) 1e+02) 1 0) (select (<= (/ (* (Variables|Default|GetBlockHealth) 1e+02) (Math|Conversions|ToFloat(Integer) (+ (stale EventBeginPlay _output_get) 1))) 75.0) 1 0) (select (<= (/ (* (Variables|Default|GetBlockHealth) 1e+02) (Math|Conversions|ToFloat(Integer) (+ (stale EventBeginPlay _output_get) 1))) 5e+01) 1 0))) :!class /Script/Engine.MaterialInstanceDynamic)
  (Variables|Default|SetBlockHealth (- (Variables|Default|GetBlockHealth) (Variables|Default|GetDamaged)))
  (if (<= (Variables|Default|GetBlockHealth) 0.0)
    ;[1 1 1] Dan's Flipbook Test Stuff
    (Components|DestroyComponent (Variables|Default|GetCube))
    (Sprite|SetFlipbook (Variables|Default|GetFlipbook%20Rock) "/Game/MineRush/ParticleSystems/ParticleFlipbooks/RockFB.RockFB")
    (Utilities|FlowControl|Delay 0.6)
    (Actor|DestroyActor)))

(fn ConstructionScript
  (if (Variables|Default|GetSmall)
    (Variables|Default|SetBlockHealth 1.0)
    (Rendering|Material|SetMaterial (Variables|Default|GetCube) 0 "/Game/MineRush/Materials/BackgroundMaster_Inst3.BackgroundMaster_Inst3")))

(fn Health
  (params (damage :type Float%20%28single-precision%29) (destoryed :type Boolean)))