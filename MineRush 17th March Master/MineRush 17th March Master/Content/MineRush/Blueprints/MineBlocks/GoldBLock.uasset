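; GoldBLock is a minable gold block that cracks under damage, then destroys itself and adds one to the damaging SideScrollerCharacter's GoldCount.
; BeginPlay creates a BackgroundMaster dynamic material, deriving Row and Column from its offset to the Is00-flagged gold block.
; AnyDamage sets Crack_Level from health before subtracting damage.
; The construction script picks rock material and health by size flags, but BeginPlay overrides both.
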(event Game|Damage|EventAnyDamage
  (params (Damage :type Float%20%28single-precision%29) (DamageType :type Damage%20Type%20Object%20Reference) (InstigatedBy :type Controller%20Object%20Reference) (DamageCauser :type Actor%20Object%20Reference))
  ;[1 1 1] Damage/Health
  (Variables|Default|SetDamaged Damage)
  ;[1 1 1] Block Crack
  (Rendering|Material|SetScalarParameterValue (stale EventBeginPlay _returnvalue_2) "Crack_Level" (Math|Conversions|ToFloat(Integer) (+ (select (<= (/ (* (Variables|Default|GetBlockHealth) 1e+02) 4.0) 1e+02) 1 0) (select (<= (/ (* (Variables|Default|GetBlockHealth) 1e+02) 4.0) 75.0) 1 0) (select (<= (/ (* (Variables|Default|GetBlockHealth) 1e+02) 4.0) 5e+01) 1 0))) :!class /Script/Engine.MaterialInstanceDynamic)
  (Variables|Default|SetBlockHealth (- (Variables|Default|GetBlockHealth) (Variables|Default|GetDamaged)))
  (if (<= (Variables|Default|GetBlockHealth) 0.0)
    (bind _asside_scroller_character (Utilities|Casting|CastToSideScrollerCharacter DamageCauser))
    (Variables|/Game/MineRush/Blueprints/Character/SideScrollerCharacter.SideScrollerCharacter_C|SetGoldCount _asside_scroller_character (+ (Variables|/Game/MineRush/Blueprints/Character/SideScrollerCharacter.SideScrollerCharacter_C|GetGoldCount _asside_scroller_character) 1))
    (Actor|DestroyActor)))

(event EventBeginPlay
  (bind _self self)
  (bind _defaultsceneroot (Variables|Default|GetDefaultSceneRoot _self))
  (bind _returnvalue (Transformation|GetWorldTransform _defaultsceneroot))
  (bind (_x _y _z) (Math|Vector|BreakVector (.location _returnvalue)))
  (Variables|Default|SetTags (Variables|Default|GetTag))
  (bind _outactors (Actor|GetAllActorsOfClass "GoldBLock_C"))
  (bind _array_element (Utilities|Array|ForEachLoopwithBreak _outactors :!label _label)
    (:LoopBody
      (if (Variables|GoldBLock_C|GetIs%2000 _array_element)
        (Variables|Default|SetGold%2000 _array_element)
        (goto _label Break)))
    (:Completed
      (Variables|Default|SetBlockHealth 4.0)
      (bind _returnvalue_2 (Rendering|Material|CreateDynamicMaterialInstance (Variables|Default|GetCube) 0 "/Game/MineRush/Materials/BackgroundMaster.BackgroundMaster" :!class /Script/Engine.PrimitiveComponent))
      (Rendering|Material|SetScalarParameterValue _returnvalue_2 "Column" (/ (- _y (.Y (Math|Vector|BreakVector (.location (Transformation|GetWorldTransform (Variables|GoldBLock_C|GetDefaultSceneRoot (Variables|Default|GetGold%2000))))))) -1e+02) :!class /Script/Engine.MaterialInstanceDynamic)
      (Rendering|Material|SetScalarParameterValue _returnvalue_2 "Row" (/ (- _z (.Z (Math|Vector|BreakVector (.location (Transformation|GetWorldTransform (Variables|GoldBLock_C|GetDefaultSceneRoot (Variables|Default|GetGold%2000))))))) -1e+02) :!class /Script/Engine.MaterialInstanceDynamic)
      (Rendering|Material|SetScalarParameterValue _returnvalue_2 "IsItAMaterial?" 1.0 :!class /Script/Engine.MaterialInstanceDynamic)
      (Rendering|Material|SetScalarParameterValue _returnvalue_2 "IsItGold" 1.0 :!class /Script/Engine.MaterialInstanceDynamic))))

(fn ConstructionScript
  (if (Variables|Default|GetSmall)
    (Variables|Default|SetBlockHealth 1.0)
    (Rendering|Material|SetMaterial (Variables|Default|GetCube) 0 "/Game/MineRush/Materials/M_MR_Rock3.M_MR_Rock3")
    (elif (Variables|Default|GetMedium)
      (Variables|Default|SetBlockHealth 2.0)
      (Rendering|Material|SetMaterial (Variables|Default|GetCube) 0 "/Game/MineRush/Materials/M_MR_Rock2.M_MR_Rock2")
      (elif (Variables|Default|GetLarge)
        (Variables|Default|SetBlockHealth 3.0)
        (Rendering|Material|SetMaterial (Variables|Default|GetCube) 0 "/Game/MineRush/Materials/M_MR_Rock1.M_MR_Rock1")))))

(fn Health
  (params (damage :type Float%20%28single-precision%29) (destoryed :type Boolean)))