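; Explosive mine block that detonates shortly after taking any damage, regardless of remaining health.
; A sphere trace damages nearby Explosives for chain reactions, destroys MineBlocks and calls StopMovement on caught SideScrollerCharacters.
; It swaps its cube for an explosion flipbook with sound, then destroys itself after a delay.
; BeginPlay creates a dynamic background material, setting grid row and column relative to the Explosive flagged Is00.
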(event Custom|Destroy%20Self%20Event
  ;[1 1 1] Dan's Flipbook Test Stuff
  (Components|DestroyComponent (Variables|Default|GetCube))
  (Sprite|SetFlipbook (Variables|Default|GetFlipbook%20Explosion) "/Game/MineRush/ParticleSystems/ParticleFlipbooks/ExploFB.ExploFB")
  (Audio|PlaySoundatLocation "/Game/MineRush/Audio/S15_DynamitePickup_2.S15_DynamitePickup_2" (Transformation|GetActorLocation))
  (Utilities|FlowControl|Delay 1.2)
  (Actor|DestroyActor))

(event EventBeginPlay
  (bind _self self)
  (bind _defaultsceneroot (Variables|Explosive_C|GetDefaultSceneRoot _self))
  (bind _returnvalue (Transformation|GetWorldTransform _defaultsceneroot))
  (bind (_x _y _z) (Math|Vector|BreakVector (.location _returnvalue)))
  (Variables|Default|SetTags (Variables|Default|GetTag))
  (bind _outactors (Actor|GetAllActorsOfClass "Explosive_C"))
  (bind _array_element (Utilities|Array|ForEachLoopwithBreak _outactors :!label _label)
    (:LoopBody
      (if (Variables|Explosive_C|GetIs%2000 _array_element)
        (Variables|Default|SetIsFirst _array_element)
        (goto _label Break)))
    (:Completed
      (bind _returnvalue_2 (Rendering|Material|CreateDynamicMaterialInstance (Variables|Default|GetCube) 0 "/Game/MineRush/Materials/BackgroundMaster.BackgroundMaster" :!class /Script/Engine.PrimitiveComponent))
      (Rendering|Material|SetScalarParameterValue _returnvalue_2 "Column" (/ (- _y (.Y (Math|Vector|BreakVector (.location (Transformation|GetWorldTransform (Variables|Explosive_C|GetDefaultSceneRoot (Variables|Default|GetIsFirst))))))) -1e+02) :!class /Script/Engine.MaterialInstanceDynamic)
      (Rendering|Material|SetScalarParameterValue _returnvalue_2 "Row" (/ (- _z (.Z (Math|Vector|BreakVector (.location (Transformation|GetWorldTransform (Variables|Explosive_C|GetDefaultSceneRoot (Variables|Default|GetIsFirst))))))) -1e+02) :!class /Script/Engine.MaterialInstanceDynamic)
      (Rendering|Material|SetScalarParameterValue _returnvalue_2 "IsItAMaterial?" 0.0 :!class /Script/Engine.MaterialInstanceDynamic))))

(event Game|Damage|EventAnyDamage
  (params (Damage :type Float%20%28single-precision%29) (DamageType :type Damage%20Type%20Object%20Reference) (InstigatedBy :type Controller%20Object%20Reference) (DamageCauser :type Actor%20Object%20Reference))
  (bind _returnvalue (Transformation|GetActorLocation))
  (bind (_x _y _z) (Math|Vector|BreakVector _returnvalue))
  (Variables|Default|SetBlockHealth (- (Variables|Default|GetBlockHealth) (Variables|Default|GetDamaged)))
  (Utilities|FlowControl|Delay 0.5)
  (bind _outhits (Class|KismetSystemLibrary|SphereTraceMultiNEW _returnvalue (Math|Vector|MakeVector _x (+ _y 0.1) _z) 1.2e+02 "TraceTypeQuery3" false 0 "None" true))
  (Utilities|FlowControl|Sequence
    (:then_0
      (bind _array_element (Utilities|Array|ForEachLoopwithBreak _outhits)
        (:LoopBody
          (bind _asexplosive (Utilities|Casting|CastToExplosive (.HitActor (Collision|BreakHitResult _array_element))))
          (Game|Damage|ApplyDamage _asexplosive 1.0 0 0))))
    (:then_1
      (CallFunction|DestroySelfEvent)
      (bind _array_element_2 (Utilities|Array|ForEachLoopwithBreak _outhits)
        (:LoopBody
          (bind _asmine_block (Utilities|Casting|CastToMineBlock (.HitActor (Collision|BreakHitResult _array_element_2))))
          (Actor|DestroyActor _asmine_block))))
    (:then_2
      (bind _array_element_3 (Utilities|Array|ForEachLoopwithBreak _outhits)
        (:LoopBody
          (bind _asside_scroller_character (Utilities|Casting|CastToSideScrollerCharacter (.HitActor (Collision|BreakHitResult _array_element_3))))
          (Default|StopMovement _asside_scroller_character))))))

(fn ConstructionScript)